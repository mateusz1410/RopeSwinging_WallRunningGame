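; BP_RunnableWall is a wall actor that tells overlapping actors they can wall-run along it.
; It has two end colliders; entering one sends a SetRunnableWallMessage with the opposite collider's location as target and its own transform as start point.
; A left/right flag differs by entry collider, so the wall works in both directions.
; Leaving either collider sends the same message with default values, disabling wall running.
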(event `self.collider1.OnComponentBeginOverlap`
  (params (OverlappedComponent :type "PrimitiveComponent Object Reference") (OtherActor :type "Actor Object Reference") (OtherComp :type "PrimitiveComponent Object Reference") (OtherBodyIndex :type Integer) (bFromSweep :type Boolean) (SweepResult :type "HitResult Structure (by ref)"))
  (message `/Game/BP/WallRun/BPI_WallRunner.setRunnableWall` OtherActor true (`SceneComponent.K2_GetComponentLocation` (`self.collider2`)) (`SceneComponent.K2_GetComponentToWorld` (`self.collider1`)) true))

(event `self.collider1.OnComponentEndOverlap`
  (params (OverlappedComponent :type "PrimitiveComponent Object Reference") (OtherActor :type "Actor Object Reference") (OtherComp :type "PrimitiveComponent Object Reference") (OtherBodyIndex :type Integer))
  (message `/Game/BP/WallRun/BPI_WallRunner.setRunnableWall` OtherActor false (0.0 0.0 0.0) (struct) false))

(event `self.collider2.OnComponentBeginOverlap`
  (params (OverlappedComponent :type "PrimitiveComponent Object Reference") (OtherActor :type "Actor Object Reference") (OtherComp :type "PrimitiveComponent Object Reference") (OtherBodyIndex :type Integer) (bFromSweep :type Boolean) (SweepResult :type "HitResult Structure (by ref)"))
  (message `/Game/BP/WallRun/BPI_WallRunner.setRunnableWall` OtherActor true (`SceneComponent.K2_GetComponentLocation` (`self.collider1`)) (`SceneComponent.K2_GetComponentToWorld` (`self.collider2`)) false))

(event `self.collider2.OnComponentEndOverlap`
  (params (OverlappedComponent :type "PrimitiveComponent Object Reference") (OtherActor :type "Actor Object Reference") (OtherComp :type "PrimitiveComponent Object Reference") (OtherBodyIndex :type Integer))
  (message `/Game/BP/WallRun/BPI_WallRunner.setRunnableWall` OtherActor false (0.0 0.0 0.0) (struct) false))

(fn `UserConstructionScript`)