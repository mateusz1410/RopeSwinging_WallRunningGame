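; BP_Rope is a swingable rope actor that the player grabs on contact.
; When a player overlaps its capsule, it messages the player to let go of any rope and grab this one, printing a debug "collision" string.
; Its AddSwingingForce event pushes CableEnd with a scaled acceleration, only while that end hangs at least 800 units below the actor's origin, which limits swing height.
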(event `self.Capsule.OnComponentBeginOverlap`
  (params (OverlappedComponent :type "PrimitiveComponent Object Reference") (OtherActor :type "Actor Object Reference") (OtherComp :type "PrimitiveComponent Object Reference") (OtherBodyIndex :type Integer) (bFromSweep :type Boolean) (SweepResult :type "HitResult Structure (by ref)"))
  (bind _yes_no (message `/Game/BP/Rope/BPI_Player.isPlayer` OtherActor))
  (if _yes_no
    (message `/Game/BP/Rope/BPI_Player.letGoRope` OtherActor)
    (`KismetSystemLibrary.PrintString` "collision" true true (`KismetMathLibrary.MakeColor` (`KismetMathLibrary.RandomFloat`) (`KismetMathLibrary.RandomFloat`) (`KismetMathLibrary.RandomFloat`)) 4.0)
    (message `/Game/BP/Rope/BPI_Player.grabRope` OtherActor self)))

(event `self.Capsule.OnComponentEndOverlap`
  (params (OverlappedComponent :type "PrimitiveComponent Object Reference") (OtherActor :type "Actor Object Reference") (OtherComp :type "PrimitiveComponent Object Reference") (OtherBodyIndex :type Integer)))

(event `Add Swinging Force`
  (params (swingForce :type "Vector Structure"))
  (bind (_returnvalue_x _returnvalue_y _returnvalue_z) (`KismetMathLibrary.BreakVector` (`self.K2_GetActorLocation`)))
  (bind (_returnvalue_x_2 _returnvalue_y_2 _returnvalue_z_2) (`KismetMathLibrary.BreakVector` (`SceneComponent.K2_GetComponentLocation` (`self.cableEnd`))))
  (if (not (< (- _returnvalue_z _returnvalue_z_2) 800.0))
    (`PrimitiveComponent.AddForce` (`self.cableEnd`) (* swingForce 500.0) "None" true)))

(fn `UserConstructionScript`)